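; Player state that persists the player's health through the Bp_gameIntense game instance and triggers respawn on death.
; On BeginPlay it loads saved health if the instance's initialized flag is set, otherwise resets the health component and writes that flag as false.
; Health component changes copy current and max health back to the instance.
; Death calls StartRespawn on BP_ThirdPersonGameMode for player controller 0.
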(event `self.ReceiveBeginPlay`
  (bind _asbp_game_intense (cast `/Game/Game/Blueprints/Bp_gameIntense` (`GameplayStatics.GetGameInstance`)))
  (bind _output_get (set `self.RefGameIntense` _asbp_game_intense))
  (if (`/Game/Game/Blueprints/Bp_gameIntense.healthInitilialized_gl` _output_get)
    (`self.loadHealthFromGameInstance`)
    (else
      (`/Game/Game/Blueprints/Components/AC_Health.ResetHealth` (`self.AC_Health`))
      (set `/Game/Game/Blueprints/Bp_gameIntense.healthInitilialized_gl` false (`self.RefGameIntense`)))))

(event `self.AC_Health.OnHealthChanged`
  (params (CurrentHealth :type "Float (double-precision)") (MaxHealth :type "Float (double-precision)"))
  (`self.saveCurrentHealth` CurrentHealth)
  (`self.saveMaxHealth` MaxHealth))

(event `self.AC_Health.OnDeath`
  (bind _asbp_third_person_game_mode (cast `/Game/Game/Blueprints/GameModes/BP_ThirdPersonGameMode` (`GameplayStatics.GetGameMode`)))
  (`/Game/Game/Blueprints/GameModes/BP_ThirdPersonGameMode.startRespawn` _asbp_third_person_game_mode (`GameplayStatics.GetPlayerController` 0)))

(fn `loadHealthFromGameInstance`
  (bind _output_get (set `/Game/Game/Blueprints/Components/AC_Health.MaxHealth` (`/Game/Game/Blueprints/Bp_gameIntense.maxHealth_gI` (`self.RefGameIntense`)) (`self.AC_Health`)))
  (bind _output_get_2 (set `/Game/Game/Blueprints/Components/AC_Health.CurrentHealth` (`/Game/Game/Blueprints/Bp_gameIntense.currentHealth_gl` (`self.RefGameIntense`)) (`self.AC_Health`)))
  (`/Game/Game/Blueprints/Components/AC_Health.OnHealthChanged` (`self.AC_Health`) _output_get_2 _output_get))

(fn `saveCurrentHealth`
  (params (NewHealth :type "Float (double-precision)"))
  (set `/Game/Game/Blueprints/Bp_gameIntense.currentHealth_gl` NewHealth (`self.RefGameIntense`)))

(fn `saveMaxHealth`
  (params (nesMaxHealth :type "Float (double-precision)"))
  (set `/Game/Game/Blueprints/Bp_gameIntense.maxHealth_gI` nesMaxHealth (`self.RefGameIntense`)))

(fn `UserConstructionScript`)